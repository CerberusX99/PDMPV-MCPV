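; Player character Blueprint that moves with Enhanced Input and can interact with, carry and drop objects.
; Interaction runs a short sphere trace in front of the character, ignoring the held object, and sends an Interact message to the hit actor.
; Grab stores the given object, attaches it to Hands and calls MoveComponentTo on its root.
; Interacting with no hit drops any held object and clears the reference.
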(event Custom|Grab
  (params (ObjectToGrab :type BP%20Grabbable%20Object%20Reference))
  ;[1 1 1] Object to actor
  (bind _output_get (Variables|Default|SetGrabObject ObjectToGrab))
  (Transformation|AttachComponentToComponent _output_get (Variables|Default|GetHands) "None" "KeepWorld" "KeepWorld" "KeepWorld" true)
  (Components|MoveComponentTo (Variables|/Script/Engine.Actor|GetRootComponent (Variables|Default|GetGrabObject)) "0, 0, 0" "0, 0, 0" false false 0.2 false))

(event Input|EnhancedActionEvents|EnhancedInputActionIA_Movement2
  (params (ActionValue :type Vector%202D%20Structure) (ElapsedSeconds :type Float%20%28double-precision%29) (TriggeredSeconds :type Float%20%28double-precision%29) (InputAction :type Input%20Action%20Object%20Reference :default "/Game/Inputs/IA_Movement2.IA_Movement2"))
  ;[1 0.1198 0.1198] Character Input Movement
  (Pawn|Input|AddMovementInput (Math|Conversions|ToVector(Vector2D) ActionValue) 1.0 false))

(event Input|EnhancedActionEvents|EnhancedInputActionNewInputAction_Interaction
  (params (ActionValue :type Boolean) (ElapsedSeconds :type Float%20%28double-precision%29) (TriggeredSeconds :type Float%20%28double-precision%29) (InputAction :type Input%20Action%20Object%20Reference :default "/Game/Inputs/NewInputAction_Interaction.NewInputAction_Interaction"))
  (bind (_returnvalue _grabobject) (CallFunction|GetGrabbedObject))
  (bind _returnvalue_2 (Transformation|GetActorForwardVector))
  (bind _returnvalue_3 (Transformation|GetActorLocation))
  (bind _returnvalue_4 (* _returnvalue_2 5e+01))
  (bind _returnvalue_5 (+ _returnvalue_4 _returnvalue_3))
  (bind (_x _y _z) (Math|Vector|BreakVector _returnvalue_5))
  ;[1 0.06771 0.06771] Character interaction
  (:Started
    (bind (_outhit _returnvalue_6) (Collision|SphereTraceByChannel (Math|Vector|MakeVector _x _y (+ _z -5e+01)) (Math|Vector|MakeVector _x _y (+ _z 1e+01)) 3e+01 "TraceTypeQuery3" false (Utilities|Array|MakeArray (Variables|Default|GetGrabObject)) "ForDuration"))
    (if _returnvalue_6
      (Class|BPIInteractable|Interact(Message) (.HitActor (Collision|BreakHitResult _outhit)) self)
      (elif _returnvalue
        (Default|Drop _grabobject)
        (Variables|Default|SetGrabObject 0)))))

(event EventBeginPlay)

(event Collision|EventActorBeginOverlap
  (params (OtherActor :type Actor%20Object%20Reference)))

(event EventTick
  (params (DeltaSeconds :type Float%20%28single-precision%29)))

(fn ConstructionScript)

(fn GetGrabbedObject
  (bind _grabobject (Variables|Default|GetGrabObject))
  (return (Utilities|IsValid _grabobject) _grabobject))